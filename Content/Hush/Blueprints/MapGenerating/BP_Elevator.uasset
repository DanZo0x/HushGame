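; BP_Elevator is the level's victory trigger, ending the game when the player character enters its box.
; The overlap calls ModifyKeyboardIMC on the player controller, then runs a delayed sequence: close the elevator door, fade to black, show the victory menu.
; It finds the door and GM_Testing with GetActorOfClass, using GM_Testing's PlayerUI for the fade.
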(event OnComponentBeginOverlap(Box)
  (params (OverlappedComponent :type Primitive%20Component%20Object%20Reference) (OtherActor :type Actor%20Object%20Reference) (OtherComp :type Primitive%20Component%20Object%20Reference) (OtherBodyIndex :type Integer) (bFromSweep :type Boolean) (SweepResult :type Hit%20Result%20Structure%20%28by%20ref%29))
  (Utilities|Casting|CastToBP_Char OtherActor)
  (Development|PrintString "Victory")
  (bind _aspc_character (Utilities|Casting|CastToPC_Character (Game|GetPlayerController 0)))
  (Default|ModifyKeyboardIMC _aspc_character)
  (Utilities|FlowControl|Delay 2.0)
  (bind _returnvalue (Actor|GetActorOfClass "/Game/Hush/Blueprints/MapGenerating/BP_ElevatorDoor.BP_ElevatorDoor_C"))
  (Default|Close _returnvalue)
  (Utilities|FlowControl|Delay 2.0)
  (bind _returnvalue_2 (Actor|GetActorOfClass "/Game/Hush/Gamemodes/GM_Testing.GM_Testing_C"))
  (Class|Image|SetOpacity (Variables|/Game/Hush/HUD/W_Crosshair.W_Crosshair_C|GetFadeBlack (Variables|/Game/Hush/Gamemodes/GM_Testing.GM_Testing_C|GetPlayerUI _returnvalue_2)) 1.0)
  (UserInterface|Animation|PlayAnimation (Variables|/Game/Hush/Gamemodes/GM_Testing.GM_Testing_C|GetPlayerUI _returnvalue_2) (Variables|/Game/Hush/HUD/W_Crosshair.W_Crosshair_C|GetFadeToBlack (Variables|/Game/Hush/Gamemodes/GM_Testing.GM_Testing_C|GetPlayerUI _returnvalue_2)) 0.0 1 "Forward" 1.0 false)
  (Utilities|FlowControl|Delay 1.0)
  (bind _returnvalue_3 (UserInterface|CreateWidget "/Game/Hush/HUD/W_VictoryMenu.W_VictoryMenu_C"))
  (UserInterface|Viewport|AddtoViewport _returnvalue_3 0))

(event EventBeginPlay)

(event Collision|EventActorBeginOverlap
  (params (OtherActor :type Actor%20Object%20Reference)))

(event EventTick
  (params (DeltaSeconds :type Float%20%28single-precision%29)))

(fn ConstructionScript)