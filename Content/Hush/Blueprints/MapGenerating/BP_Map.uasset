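; BP_Map builds a randomized 3x3 map at BeginPlay and handles monster placement.
; It moves random pre-placed corner (Coin), side and center zones into rotated grid slots, then destroys unused ones.
; It removes stray lights, swaps crouch-light markers for BP_CrouchGatesLight, positions the floor and plays a hum.
; eventSpawnMonster teleports the existing monster to a random corner zone's child actor far from the player, with an attached scream.
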(event Custom|eventSpawnMonster
  (for _array_element (Variables|Default|GetCoinsOfMap)
    (if (not (< (Math|Vector|Distance(Vector) (Transformation|GetActorLocation (Variables|/Script/Engine.ChildActorComponent|GetChildActor (Actor|GetComponentbyClass _array_element "/Script/Engine.ChildActorComponent"))) (Transformation|GetActorLocation (Game|GetPlayerCharacter 0))) (Variables|Default|GetDistFromPlayer)))
      (Utilities|Array|Add (Variables|Default|GetCoinsFarAwayFromPlayer) _array_element)))
  (bind _returnvalue (Actor|GetActorOfClass "/Game/Hush/Blueprints/IA/BP_Monstre.BP_Monstre_C"))
  (Transformation|SetActorLocation _returnvalue (Transformation|GetActorLocation (Variables|/Script/Engine.ChildActorComponent|GetChildActor (Actor|GetComponentbyClass (.OutItem (Utilities|Array|Random (Variables|Default|GetCoinsFarAwayFromPlayer))) "/Script/Engine.ChildActorComponent"))) false false)
  (Audio|SpawnSoundAttached "/Game/Hush/Sound/Monster/Monster_scream_loin_1_echofort_fixed.Monster_scream_loin_1_echofort_fixed" (Actor|GetComponentbyClass _returnvalue "/Script/Engine.AudioComponent") "None" "0, 0, 0" "0, 0, 0" "KeepRelativeOffset" false 1.0 1.0 0.0 0 0))

(event EventBeginPlay
  (bind _outactors (Actor|GetAllActorsOfClass "/Game/Hush/Blueprints/MapGenerating/Zones/BP_Coin.BP_Coin_C"))
  (for _array_element _outactors
    (Utilities|Array|Add (Variables|Default|GetArrayCoins) _array_element))
  (bind _outactors_2 (Actor|GetAllActorsOfClass "/Game/Hush/Blueprints/MapGenerating/Zones/BP_Center.BP_Center_C"))
  (for _array_element_2 _outactors_2
    (Utilities|Array|Add (Variables|Default|GetArrayCenter) _array_element_2))
  (bind _outactors_3 (Actor|GetAllActorsOfClass "/Game/Hush/Blueprints/MapGenerating/Zones/BP_Side.BP_Side_C"))
  (for _array_element_3 _outactors_3
    (Utilities|Array|Add (Variables|Default|GetArraySide) _array_element_3))
  (for _index (range 0 2)
    (Variables|Default|SetXLocation (+ (Variables|Default|GetXLocation) 4.1e+03))
    (Variables|Default|SetYLocation -4.1e+03)
    (for _index_2 (range 0 2)
      (switch int (Variables|Default|GetCaseID)
        (:0
          (Variables|Default|SetRotationAngleCoin 0.0)
          (bind _output_get (Variables|Default|SetTemp_Zone (.OutItem (Utilities|Array|Random (Variables|Default|GetArrayCoins))) :!label _label))
          (bind _asbp_coin (Utilities|Casting|CastToBP_Coin _output_get))
          (Rendering|SetActorHiddenInGame _output_get false)
          (Transformation|SetActorLocation _output_get (Math|Vector|MakeVector (Variables|Default|GetXLocation) (Variables|Default|GetYLocation) -1e+02) false false)
          (Transformation|SetActorRotation _output_get (Math|Rotator|MakeRotator 0.0 0.0 (Variables|Default|GetRotationAngleCoin)))
          (Variables|/Game/Hush/Blueprints/MapGenerating/Zones/BP_Zone.BP_Zone_C|SetIsCoin (Variables|Default|GetTemp_Zone) true)
          (Utilities|Array|RemoveItem (Variables|Default|GetArrayCoins) _asbp_coin)
          (Utilities|Array|Add (Variables|Default|GetCoinsOfMap) _output_get))
        (:1
          (Variables|Default|SetRotationAngleSide 0.0)
          (bind _output_get_2 (Variables|Default|SetTemp_Zone (.OutItem (Utilities|Array|Random (Variables|Default|GetArraySide))) :!label _label_2))
          (bind _asbp_side (Utilities|Casting|CastToBP_Side _output_get_2))
          (Rendering|SetActorHiddenInGame _output_get_2 false)
          (Transformation|SetActorLocation _output_get_2 (Math|Vector|MakeVector (Variables|Default|GetXLocation) (Variables|Default|GetYLocation) -1e+02) false false)
          (Transformation|SetActorRotation _output_get_2 (Math|Rotator|MakeRotator 0.0 0.0 (Variables|Default|GetRotationAngleSide)))
          (Variables|/Game/Hush/Blueprints/MapGenerating/Zones/BP_Zone.BP_Zone_C|SetIsSide (Variables|Default|GetTemp_Zone) true)
          (Utilities|Array|RemoveItem (Variables|Default|GetArraySide) _asbp_side))
        (:2
          (Variables|Default|SetRotationAngleCoin 2.7e+02)
          (goto _label))
        (:3
          (Variables|Default|SetRotationAngleSide 9e+01)
          (goto _label_2))
        (:4
          (bind _output_get_3 (Variables|Default|SetTemp_Zone (.OutItem (Utilities|Array|Random (Variables|Default|GetArrayCenter)))))
          (bind _asbp_center (Utilities|Casting|CastToBP_Center _output_get_3))
          (Rendering|SetActorHiddenInGame _output_get_3 false)
          (Transformation|SetActorLocation _output_get_3 (Math|Vector|MakeVector (Variables|Default|GetXLocation) (Variables|Default|GetYLocation) -1e+02) false false)
          (Variables|/Game/Hush/Blueprints/MapGenerating/Zones/BP_Zone.BP_Zone_C|SetIsCenter (Variables|Default|GetTemp_Zone) true)
          (Utilities|Array|RemoveItem (Variables|Default|GetArrayCenter) _asbp_center))
        (:5
          (Variables|Default|SetRotationAngleSide 2.7e+02)
          (goto _label_2))
        (:6
          (Variables|Default|SetRotationAngleCoin 9e+01)
          (goto _label))
        (:7
          (Variables|Default|SetRotationAngleSide 1.8e+02)
          (goto _label_2))
        (:8
          (Variables|Default|SetRotationAngleCoin 1.8e+02)
          (goto _label)))
      (Variables|Default|SetYLocation (+ (Variables|Default|GetYLocation) 4.1e+03))
      (Math|Integer|IncrementInt (Variables|Default|GetCaseID))))
  (for _array_element_4 (Variables|Default|GetArrayCoins)
    (Actor|DestroyActor _array_element_4))
  (for _array_element_5 (Variables|Default|GetArraySide)
    (Actor|DestroyActor _array_element_5))
  (for _array_element_6 (Variables|Default|GetArrayCenter)
    (Actor|DestroyActor _array_element_6))
  (bind _outactors_4 (Actor|GetAllActorsOfClass "/Game/Hush/Blueprints/MapGenerating/Light/BP_LightMap.BP_LightMap_C"))
  (for _array_element_7 _outactors_4
    (Utilities|Casting|CastToBP_Zone (Actor|GetAttachParentActor _array_element_7)
      (:CastFailed
        (Actor|DestroyActor _array_element_7))))
  (bind _outactors_5 (Actor|GetAllActorsOfClass "/Game/Hush/Blueprints/MapGenerating/Light/BP_PointCrounchLight.BP_PointCrounchLight_C"))
  (for _array_element_8 _outactors_5
    (Utilities|Casting|CastToBP_Zone (Actor|GetAttachParentActor _array_element_8)
      (:then
        (Game|SpawnActorfromClass "/Game/Hush/Blueprints/MapGenerating/Light/BP_CrouchGatesLight.BP_CrouchGatesLight_C" (Math|Transform|MakeTransform (Transformation|GetActorLocation _array_element_8) "0, 0, 0" "1.000000,1.000000,1.000000") "Undefined" 0 0))
      (:CastFailed
        (Actor|DestroyActor _array_element_8))))
  (bind _outactors_6 (Actor|GetAllActorsOfClass "/Game/Hush/Blueprints/MapGenerating/Light/BP_PointCrounchLight.BP_PointCrounchLight_C"))
  (for _array_element_9 _outactors_6
    (Actor|DestroyActor _array_element_9))
  (bind _returnvalue (Actor|GetActorOfClass "/Game/Hush/Blueprints/MapGenerating/BP_Floor.BP_Floor_C"))
  (Transformation|SetActorLocation _returnvalue "0.000000,0.000000,350.000000" false false)
  (Audio|PlaySound2D "/Game/Hush/Sound/low_huming_long.low_huming_long" 1.0 1.0 0.0 0 0))

(fn ConstructionScript)