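; Interactable gramophone that the player switches on to play a positional sound and report a loud noise event for AI hearing.
; Tick shows an interact widget and enables the interact input context while external detection events and box overlap both flag the player as able to interact.
; Switching on disables that input and sets a playing flag, which suppresses the prompt until a fixed delay clears it.
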(event OnComponentBeginOverlap(Box)
  (params (OverlappedComponent :type Primitive%20Component%20Object%20Reference) (OtherActor :type Actor%20Object%20Reference) (OtherComp :type Primitive%20Component%20Object%20Reference) (OtherBodyIndex :type Integer) (bFromSweep :type Boolean) (SweepResult :type Hit%20Result%20Structure%20%28by%20ref%29))
  (Utilities|Casting|CastToBP_Char OtherActor)
  (Variables|Default|SetIsInRange true))

(event OnComponentEndOverlap(Box)
  (params (OverlappedComponent :type Primitive%20Component%20Object%20Reference) (OtherActor :type Actor%20Object%20Reference) (OtherComp :type Primitive%20Component%20Object%20Reference) (OtherBodyIndex :type Integer))
  (Utilities|Casting|CastToBP_Char OtherActor)
  (Variables|Default|SetIsInRange false))

(event Custom|SwitchOnGramophone
  (bind _aspc_character (Utilities|Casting|CastToPC_Character (Game|GetPlayerController 0)))
  (Default|ModifyInteractIMC _aspc_character false)
  (Class|AISenseHearing|ReportNoiseEvent (Transformation|GetActorLocation) 3.0 self 0.0 "None")
  (bind _returnvalue (Audio|SpawnSoundatLocation "/Game/Hush/Sound/Objects/Gramophone/Peppa_Pig_｜_Générique_｜_NICKELODEON_JUNIOR.Peppa_Pig_｜_Générique_｜_NICKELODEON_JUNIOR" (Transformation|GetActorLocation) "0, 0, 0" 1.0 1.0 0.0 "/Game/Hush/Sound/Objects/Gramophone/SA_Gramophone.SA_Gramophone" 0))
  (Variables|Default|SetLever%20Sound _returnvalue)
  (Variables|Default|SetSoundIsPlaying true)
  (Utilities|FlowControl|Delay 16.0)
  (Variables|Default|SetSoundIsPlaying false))

(event Custom|GramophoneNotDetected
  (Variables|Default|SetIsDetected false))

(event Custom|GramophoneIsDetected
  (Variables|Default|SetIsDetected true))

(event EventTick
  (params (DeltaSeconds :type Float%20%28single-precision%29))
  (if (Variables|Default|GetSoundIsPlaying)
    (Widget|RemovefromParent (Variables|Default|GetWidgetHold))
    (Variables|Default|SetWidgetIsActive false)
    (elif (and (Variables|Default|GetIsDetected) (Variables|Default|GetIsInRange))
      (if (not (Variables|Default|GetWidgetIsActive))
        (bind _returnvalue (UserInterface|CreateWidget "/Game/Hush/HUD/W_Interact.W_Interact_C"))
        (bind _output_get (Variables|Default|SetWidgetHold _returnvalue))
        (UserInterface|Viewport|AddtoViewport _output_get 0)
        (Variables|Default|SetWidgetIsActive true)
        (Default|ModifyInteractIMC (Variables|Default|GetPC_Character) true))
      (elif (Variables|Default|GetWidgetIsActive)
        (Widget|RemovefromParent (Variables|Default|GetWidgetHold))
        (Variables|Default|SetWidgetIsActive false)
        (Default|ModifyInteractIMC (Variables|Default|GetPC_Character) false)))))

(event EventBeginPlay
  (bind _aspc_character (Utilities|Casting|CastToPC_Character (Game|GetPlayerController 0)))
  (Variables|Default|SetPC_Character _aspc_character)
  (bind _returnvalue (Actor|GetActorOfClass "/Game/Hush/Gamemodes/GM_Testing.GM_Testing_C"))
  (Variables|Default|SetAs%20GM%20Testing _returnvalue))

(fn ConstructionScript)