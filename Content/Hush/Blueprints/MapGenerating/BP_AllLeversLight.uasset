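; BP_AllLeversLight is a four-light indicator that shows how many levers have been pulled.
; ChangeLight switches on the pulled count (1 to 4), updating only the matching light mesh and point light.
; It applies the RedLightLever material to the mesh but turns the point light green, despite that material's name.
; BeginPlay caches the GM_Testing game mode, though nothing in this graph uses it.
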(event Custom|ChangeLight
  (params (NumberOfLeverPulled :type Integer))
  (switch int NumberOfLeverPulled
    (:1
      (Rendering|Material|SetMaterial (Variables|Default|GetLight1) 0 "/Game/Hush/Material/RedLightLever.RedLightLever")
      (Rendering|Components|Light|SetLightColor (Variables|Default|GetPointLight1) (Class|KismetMathLibrary|LinearColorGreen) true))
    (:2
      (Rendering|Material|SetMaterial (Variables|Default|GetLight2) 0 "/Game/Hush/Material/RedLightLever.RedLightLever")
      (Rendering|Components|Light|SetLightColor (Variables|Default|GetPointLight2) (Class|KismetMathLibrary|LinearColorGreen) true))
    (:3
      (Rendering|Material|SetMaterial (Variables|Default|GetLight3) 0 "/Game/Hush/Material/RedLightLever.RedLightLever")
      (Rendering|Components|Light|SetLightColor (Variables|Default|GetPointLight3) (Class|KismetMathLibrary|LinearColorGreen) true))
    (:4
      (Rendering|Material|SetMaterial (Variables|Default|GetLight4) 0 "/Game/Hush/Material/RedLightLever.RedLightLever")
      (Rendering|Components|Light|SetLightColor (Variables|Default|GetPointLight4) (Class|KismetMathLibrary|LinearColorGreen) true))))

(event EventBeginPlay
  (bind _asgm_testing (Utilities|Casting|CastToGM_Testing (Game|GetGameMode)))
  (Variables|Default|SetAs%20GM%20Testing _asgm_testing))

(fn ConstructionScript)