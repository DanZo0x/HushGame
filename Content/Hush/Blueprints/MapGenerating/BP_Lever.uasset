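; BP_Lever is a hold-to-interact lever that counts toward a level's lever total in GM_Testing.
; Tick shows W_LeverInteract and enables hold interaction on PC_Character while the lever is detected and BP_Char overlaps its box, removing both otherwise.
; External events flag detection, advance the widget's hold time, and increment LeversUsed on completion.
; IsDetected and WidgetIsActive are never cleared here, and reaching LeversNeeded triggers nothing yet.
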(event OnComponentBeginOverlap(Box)
  (params (OverlappedComponent :type Primitive%20Component%20Object%20Reference) (OtherActor :type Actor%20Object%20Reference) (OtherComp :type Primitive%20Component%20Object%20Reference) (OtherBodyIndex :type Integer) (bFromSweep :type Boolean) (SweepResult :type Hit%20Result%20Structure%20%28by%20ref%29))
  (Utilities|Casting|CastToBP_Char OtherActor)
  (Variables|Default|SetIsInRange true))

(event OnComponentEndOverlap(Box)
  (params (OverlappedComponent :type Primitive%20Component%20Object%20Reference) (OtherActor :type Actor%20Object%20Reference) (OtherComp :type Primitive%20Component%20Object%20Reference) (OtherBodyIndex :type Integer))
  (Utilities|Casting|CastToBP_Char OtherActor)
  (Variables|Default|SetIsInRange false))

(event Custom|LeverDetected
  (Variables|Default|SetIsDetected true))

(event Custom|UpdateHoldWidget
  (bind _widgethold (Variables|Default|GetWidgetHold))
  (Variables|/Game/Hush/HUD/W_LeverInteract.W_LeverInteract_C|SetTimeHeld _widgethold (+ (Variables|/Game/Hush/HUD/W_LeverInteract.W_LeverInteract_C|GetTimeHeld _widgethold) 0.06525)))

(event Custom|EndHoldingLever
  (bind _as_gm_testing (Variables|Default|GetAs_GM_Testing))
  (Variables|/Game/Hush/Gamemodes/GM_Testing.GM_Testing_C|SetLeversUsed _as_gm_testing (+ (Variables|/Game/Hush/Gamemodes/GM_Testing.GM_Testing_C|GetLeversUsed _as_gm_testing) 1))
  (if (== (Variables|/Game/Hush/Gamemodes/GM_Testing.GM_Testing_C|GetLeversUsed _as_gm_testing) (Variables|/Game/Hush/Gamemodes/GM_Testing.GM_Testing_C|GetLeversNeeded _as_gm_testing))
    _))

(event EventTick
  (params (DeltaSeconds :type Float%20%28single-precision%29))
  (if (and (Variables|Default|GetIsDetected) (Variables|Default|GetIsInRange))
    (if (not (Variables|Default|GetWidgetIsActive))
      (bind _returnvalue (UserInterface|CreateWidget "/Game/Hush/HUD/W_LeverInteract.W_LeverInteract_C"))
      (bind _output_get (Variables|Default|SetWidgetHold _returnvalue))
      (UserInterface|Viewport|AddtoViewport _output_get 0)
      (Variables|Default|SetWidgetIsActive true)
      (Variables|/Game/Hush/PlayerController/PC_Character.PC_Character_C|SetCanHoldInteract (Variables|Default|GetPC_Character) true))
    (elif (Variables|Default|GetWidgetIsActive)
      (Widget|RemovefromParent (Variables|Default|GetWidgetHold))
      (Variables|/Game/Hush/PlayerController/PC_Character.PC_Character_C|SetCanHoldInteract (Variables|Default|GetPC_Character) false))))

(event EventBeginPlay
  (bind _aspc_character (Utilities|Casting|CastToPC_Character (Game|GetPlayerController 0)))
  (Variables|Default|SetPC_Character _aspc_character)
  (bind _returnvalue (Actor|GetActorOfClass "/Game/Hush/Gamemodes/GM_Testing.GM_Testing_C"))
  (Variables|Default|SetAs_GM_Testing _returnvalue))

(fn ConstructionScript)