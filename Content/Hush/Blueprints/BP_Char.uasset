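; Player character for Hush that drives monster-proximity audio and a light flash ability.
; Every Tick it finds BP_Monster and scales heartbeat volume and pitch in distance bands, stopping it on death.
; At close range, being seen by the monster sets chase state, mutes the monster's audio and toggles its chase loop.
; The flash plays a sound, reports AI noise, and spikes then fades the spotlight through a Delay loop before re-enabling.
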(event Custom|eventFlash
  (bind _returnvalue (Game|GetPlayerCharacter 0))
  (bind _returnvalue_2 (Transformation|GetActorLocation _returnvalue))
  (if (Variables|Default|GetCanActivate)
    (Audio|PlaySoundatLocation "/Game/Hush/Sound/Player/flash.flash" _returnvalue_2 "0, 0, 0" 1.0 1.0 0.0 0 0 0 0)
    (Class|AISenseHearing|ReportNoiseEvent _returnvalue_2 2.0 _returnvalue 0.0 "None")
    (Variables|Default|SetIntensity 1.6e+05)
    (Rendering|Components|Light|SetIntensity (Variables|Default|GetSpotLight) (Variables|Default|GetIntensity))
    (Utilities|FlowControl|Delay 0.1)
    (if (>= (Variables|Default|GetIntensity) 0.0) :!label _label
      (Variables|Default|SetCanActivate false)
      (Variables|Default|SetIntensity (- (Variables|Default|GetIntensity) 1.2e+04))
      (Rendering|Components|Light|SetIntensity (Variables|Default|GetSpotLight) (Variables|Default|GetIntensity))
      (Utilities|FlowControl|Delay 0.02)
      (goto _label)
      (else
        (Utilities|FlowControl|Delay 1.0)
        (Variables|Default|SetCanActivate true)))))

(event EventTick
  (params (DeltaSeconds :type Float%20%28single-precision%29))
  (if (Variables|Default|GetIsDead)
    (Utilities|IsValid (Variables|Default|GetHeartBeatSound)
      (:Is%20Valid
        (Audio|Components|Audio|Stop (Variables|Default|GetHeartBeatSound))))
    (else
      (bind _returnvalue (Actor|GetActorOfClass "/Game/Hush/Blueprints/AIMonstreTest/BP_Monster.BP_Monster_C"))
      (Utilities|IsValid _returnvalue
        (:Is%20Valid
          (bind _output_get (Variables|Default|SetDistance (Math|Vector|Distance(Vector) (Transformation|GetActorLocation) (Transformation|GetActorLocation _returnvalue))))
          (if (< _output_get 3e+03)
            (if (< (Variables|Default|GetDistance) 2e+03)
              (if (< (Variables|Default|GetDistance) 1e+03)
                (Audio|Components|Audio|SetVolumeMultiplier (Variables|Default|GetHeartBeatSound) 1.3 :!class /Script/Engine.AudioComponent)
                (Audio|Components|Audio|SetPitchMultiplier (Variables|Default|GetHeartBeatSound) 1.5)
                (if (Variables|Default|GetIsSeenByMonster)
                  (if (not (Variables|Default|GetChaseSoundPlaying))
                    (bind _returnvalue_2 (Actor|GetActorOfClass "/Game/Hush/Blueprints/AIMonstreTest/BP_Monster.BP_Monster_C"))
                    (Audio|Components|Audio|SetVolumeMultiplier (Variables|/Game/Hush/Blueprints/AIMonstreTest/BP_Monster.BP_Monster_C|GetMonstreAudio _returnvalue_2) 0.0 :!class /Script/Engine.AudioComponent)
                    (Variables|Default|SetChaseSoundPlaying true)
                    (Variables|Default|SetIsInChase true)
                    (bind _returnvalue_3 (Actor|GetActorOfClass "/Game/Hush/Blueprints/AIMonstreTest/BP_Monster.BP_Monster_C" :!label _label))
                    (Default|ChaseLoopAudioManager _returnvalue_3 (Variables|Default|GetChaseSoundPlaying)))
                  (else
                    (bind _returnvalue_4 (Actor|GetActorOfClass "/Game/Hush/Blueprints/AIMonstreTest/BP_Monster.BP_Monster_C"))
                    (Audio|Components|Audio|SetVolumeMultiplier (Variables|/Game/Hush/Blueprints/AIMonstreTest/BP_Monster.BP_Monster_C|GetMonstreAudio _returnvalue_4) 1.0 :!class /Script/Engine.AudioComponent)
                    (Variables|Default|SetChaseSoundPlaying false)
                    (Variables|Default|SetIsInChase false)
                    (goto _label)))
                (else
                  (Audio|Components|Audio|SetVolumeMultiplier (Variables|Default|GetHeartBeatSound) 1.0 :!class /Script/Engine.AudioComponent)
                  (Audio|Components|Audio|SetPitchMultiplier (Variables|Default|GetHeartBeatSound) 1.2)
                  (Variables|Default|SetIsInChase false :!label _label_2)
                  (Variables|Default|SetChaseSoundPlaying false)
                  (bind _returnvalue_5 (Actor|GetActorOfClass "/Game/Hush/Blueprints/AIMonstreTest/BP_Monster.BP_Monster_C"))
                  (Default|ChaseLoopAudioManager _returnvalue_5 false)))
              (elif (Variables|Default|GetHeartBeatPlaying)
                (Audio|Components|Audio|SetVolumeMultiplier (Variables|Default|GetHeartBeatSound) 0.5 :!class /Script/Engine.AudioComponent)
                (Audio|Components|Audio|SetPitchMultiplier (Variables|Default|GetHeartBeatSound) 1.0)
                (else
                  (Variables|Default|SetHeartBeatPlaying true)
                  (bind _returnvalue_6 (Audio|SpawnSound2D "/Game/Hush/Sound/Player/Player_Heartbeat_Sound_Effect.Player_Heartbeat_Sound_Effect" 0.5 1.0 0.0 0))
                  (bind _output_get_2 (Variables|Default|SetHeartBeatSound _returnvalue_6))
                  (Audio|Components|Audio|FadeIn _output_get_2 0.5 1.0 0.0 "Linear" :!class /Script/Engine.AudioComponent)
                  (goto _label_2))))
            (else
              (Utilities|IsValid (Variables|Default|GetHeartBeatSound)
                (:Is%20Valid
                  (Audio|Components|Audio|FadeOut (Variables|Default|GetHeartBeatSound) 0.5 0.0 "Linear" :!class /Script/Engine.AudioComponent)
                  (Variables|Default|SetHeartBeatPlaying false)
                  (goto _label_2))))))))))

(fn ConstructionScript)