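; AI controller for the monster, running BT_Monster and feeding sight and hearing perception into its Blackboard.
; Sight sets the player as TargetActor, or clears it and records LastKnownLocation when sight is lost.
; Hearing stores the noise position in TargetLocation, plays an alert sound at the monster and sets its walk speed.
; The monster is found through GetActorOfClass rather than the controlled pawn, so a single BP_Monster is assumed.
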(event OnTargetPerceptionUpdated(AIPerception)
  (params (Actor :type Actor%20Object%20Reference) (Stimulus :type AI%20Stimulus%20Structure))
  (CallFunction|HandleSightSense Actor Stimulus)
  (CallFunction|HandleSoundSense Stimulus))

(event EventBeginPlay
  (AI|RunBehaviorTree "/Game/Hush/Blueprints/AIMonstreTest/BT_Monster.BT_Monster"))

(event EventTick
  (params (DeltaSeconds :type Float%20%28single-precision%29)))

(fn ConstructionScript)

(fn HandleSightSense
  (params (Actor :type Actor%20Object%20Reference) (Stimulus :type AI%20Stimulus%20Structure))
  (bind _returnvalue (Class|AIPerceptionSystem|GetSenseClassforStimulus Stimulus))
  (if (== _returnvalue "/Script/AIModule.AISense_Sight")
    (if (== Actor (Game|GetPlayerCharacter 0))
      (AI|Components|Blackboard|SetValueasObject (Variables|Default|GetBlackboard) (Utilities|Name|MakeLiteralName "TargetActor") (Utilities|SelectObject (Game|GetPlayerCharacter 0) 0 (.bsuccessfullysensed Stimulus)))
      (Development|PrintString "Hello")
      (if (not (.bsuccessfullysensed Stimulus))
        (AI|Components|Blackboard|SetValueasVector (Variables|Default|GetBlackboard) (Utilities|Name|MakeLiteralName "LastKnownLocation") (.stimuluslocation Stimulus)))
      (else
        (return)))
    (else
      (return))))

(fn HandleSoundSense
  (params (Stimulus :type AI%20Stimulus%20Structure%20%28by%20ref%29))
  (bind _returnvalue (Class|AIPerceptionSystem|GetSenseClassforStimulus Stimulus))
  (if (== _returnvalue "/Script/AIModule.AISense_Hearing")
    (AI|Components|Blackboard|SetValueasVector (Variables|Default|GetBlackboard) (Utilities|Name|MakeLiteralName "TargetLocation") (.StimulusLocation (Utilities|Struct|BreakAIStimulus Stimulus)))
    (bind _returnvalue_2 (Actor|GetActorOfClass "/Game/Hush/Blueprints/AIMonstreTest/BP_Monster.BP_Monster_C"))
    (Audio|PlaySoundatLocation "/Game/Hush/Sound/Monster/ALERTE.ALERTE" (Transformation|GetActorLocation _returnvalue_2) "0, 0, 0" 1.0 1.0 0.0 "/Game/Hush/Sound/Monster/SA_MonsterBigRange.SA_MonsterBigRange" 0 0 0)
    (Variables|/Script/Engine.CharacterMovementComponent|SetMaxWalkSpeed (Actor|GetComponentbyClass _returnvalue_2 "/Script/Engine.CharacterMovementComponent") 6e+02)))