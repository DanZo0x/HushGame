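; BP_Monster is the monster character, handling its spawn and chase audio and its movement speed.
; On spawn it plays an attached distant scream, then after a delay switches that component to short-range attenuation and the SC_Monster sound.
; ChaseLoopAudioManager fades an attached chase loop in or out, using a flag to prevent duplicate playback.
; AddSpeedMonster raises max walk speed and prints the result.
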(event Custom|MonsterSpawned
  (bind _returnvalue (Audio|SpawnSoundAttached "/Game/Hush/Sound/Monster/Monster_scream_loin_1_echofort_fixed.Monster_scream_loin_1_echofort_fixed" (Variables|Default|GetMonsterAudioComponent) "None" "0, 0, 0" "0, 0, 0" "KeepRelativeOffset" false 0.7 1.0 0.0 0 0))
  (Variables|Default|SetMonstreAudio _returnvalue)
  (Utilities|FlowControl|Delay 9.0)
  (Variables|/Script/Engine.AudioComponent|SetAttenuationSettings (Variables|Default|GetMonstreAudio) "/Game/Hush/Sound/Monster/SA_MonsterLittleRange.SA_MonsterLittleRange")
  (Audio|Components|Audio|SetSound (Variables|Default|GetMonstreAudio) "/Game/Hush/Sound/Monster/SC_Monster.SC_Monster"))

(event Custom|ChaseLoopAudioManager
  (params (IsActive :type Boolean))
  (if IsActive
    (if (not (Variables|Default|GetChaseLoopIsPlaying))
      (bind _returnvalue (Audio|SpawnSoundAttached "/Game/Hush/Sound/Monster/Monster_scream_chase_loop.Monster_scream_chase_loop" (Variables|Default|GetChaseAudioComponent) "None" "0, 0, 0" "0, 0, 0" "KeepRelativeOffset" false 1.0 1.0 0.0 "/Game/Hush/Sound/Monster/SA_MonsterLittleRange.SA_MonsterLittleRange" 0))
      (bind _output_get (Variables|Default|SetChaseAudio _returnvalue))
      (Audio|Components|Audio|FadeIn _output_get 0.3 1.0 0.0 "Linear" :!class /Script/Engine.AudioComponent)
      (Variables|Default|SetChaseLoopIsPlaying true))
    (else
      (Utilities|IsValid (Variables|Default|GetChaseAudio)
        (:Is%20Valid
          (Audio|Components|Audio|FadeOut (Variables|Default|GetChaseAudio) 0.3 0.0 "Linear" :!class /Script/Engine.AudioComponent)
          (Variables|Default|SetChaseLoopIsPlaying false)
          (Variables|Default|SetStartChaseHasBeenPlayed false))))))

(event Custom|AddSpeedMonster
  (params (SpeedToAdd :type Float%20%28double-precision%29))
  (bind _charactermovement (Variables|Character|GetCharacterMovement))
  (bind _output_get (Variables|/Script/Engine.CharacterMovementComponent|SetMaxWalkSpeed _charactermovement (+ (Variables|/Script/Engine.CharacterMovementComponent|GetMaxWalkSpeed _charactermovement) SpeedToAdd)))
  (Development|PrintString (Utilities|String|ToString(Float) _output_get)))

(fn ConstructionScript)