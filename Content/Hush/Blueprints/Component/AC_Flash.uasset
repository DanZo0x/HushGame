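; AC_Flash is a component that fires a camera-style flash from the player character, with a sound and an AI noise event.
; The flash event finds the spotlight at a fixed child index under the player's capsule and spikes its intensity.
; A delay loop then steps the intensity down to fade the burst.
; A CanActivate flag blocks re-firing until the fade and a short cooldown finish.
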(event Custom|eventFlash
  (bind _returnvalue (Game|GetPlayerCharacter 0))
  (bind _returnvalue_2 (Transformation|GetActorLocation _returnvalue))
  (if (Variables|Default|GetCanActivate)
    (Audio|PlaySoundatLocation "/Game/Hush/Sound/Player/flash.flash" _returnvalue_2 "0, 0, 0" 1.0 1.0 0.0 0 0 0 0)
    (Class|AISenseHearing|ReportNoiseEvent _returnvalue_2 1.0 _returnvalue 0.0 "None")
    (Variables|Default|SetIntensity 1.6e+05)
    (bind _asspot_light_component (Utilities|Casting|CastToSpotLightComponent (Components|GetChildComponent (Variables|/Script/Engine.Character|GetCapsuleComponent (Game|GetPlayerCharacter 0)) 3)))
    (bind _output_get (Variables|Default|SetAsSpotLightComponent _asspot_light_component))
    (Rendering|Components|Light|SetIntensity _asspot_light_component (Variables|Default|GetIntensity))
    (Utilities|FlowControl|Delay 0.1)
    (if (>= (Variables|Default|GetIntensity) 0.0) :!label _label
      (Variables|Default|SetCanActivate false)
      (Variables|Default|SetIntensity (- (Variables|Default|GetIntensity) 1.2e+04))
      (Rendering|Components|Light|SetIntensity (Variables|Default|GetAsSpotLightComponent) (Variables|Default|GetIntensity))
      (Utilities|FlowControl|Delay 0.02)
      (goto _label)
      (else
        (Utilities|FlowControl|Delay 1.0)
        (Variables|Default|SetCanActivate true)))))