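; GM_Testing is a game mode that handles level progression and end states through its events.
; When all levers are activated, it opens the elevator door and plays the opening sound at the door.
; Victory and defeat fade the player UI to black before showing their menus; victory also fades out the elevator sound and loads the main menu.
; BeginPlay also turns on on-screen debug messages.
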(event Custom|AllLeversActivated
  (bind _returnvalue (Actor|GetActorOfClass "/Game/Hush/Blueprints/MapGenerating/BP_ElevatorDoor.BP_ElevatorDoor_C"))
  (Default|Open _returnvalue)
  (Audio|PlaySoundatLocation "/Game/Hush/Sound/Objects/Elevator/Elevator_openning.Elevator_openning" (Transformation|GetActorLocation _returnvalue) "0, 0, 0" 1.0 1.0 0.0 "/Game/Hush/Sound/Objects/Elevator/SA_ElevatorDoor.SA_ElevatorDoor" 0 0 0))

(event Custom|VictoryScreen
  (bind _playerui (Variables|Default|GetPlayerUI))
  (Class|Image|SetOpacity (Variables|/Game/Hush/HUD/W_Crosshair.W_Crosshair_C|GetFadeBlack _playerui) 1.0)
  (UserInterface|Animation|PlayAnimation _playerui (Variables|/Game/Hush/HUD/W_Crosshair.W_Crosshair_C|GetFadeToBlack _playerui) 0.0 1 "Forward" 1.0 false)
  (Utilities|FlowControl|Delay 2.0)
  (bind _returnvalue (UserInterface|CreateWidget "/Game/Hush/HUD/W_VictoryMenu.W_VictoryMenu_C"))
  (UserInterface|Viewport|AddtoViewport _returnvalue 0)
  (bind _returnvalue_2 (Actor|GetActorOfClass "/Game/Hush/Blueprints/MapGenerating/BP_Elevator.BP_Elevator_C"))
  (Audio|Components|Audio|FadeOut (Variables|/Game/Hush/Blueprints/MapGenerating/BP_Elevator.BP_Elevator_C|GetElevatorSound _returnvalue_2) 2.0 0.0 "Linear" :!class /Script/Engine.AudioComponent)
  (Utilities|FlowControl|Delay 2.0)
  (Game|OpenLevel(byObjectReference) "/Game/Hush/Levels/MainMenu.MainMenu"))

(event Custom|DefeatScreen
  (bind _playerui (Variables|Default|GetPlayerUI))
  (Class|Image|SetOpacity (Variables|/Game/Hush/HUD/W_Crosshair.W_Crosshair_C|GetFadeBlack _playerui) 1.0)
  (UserInterface|Animation|PlayAnimation _playerui (Variables|/Game/Hush/HUD/W_Crosshair.W_Crosshair_C|GetFadeToBlack _playerui) 0.0 1 "Forward" 1.0 false)
  (Utilities|FlowControl|Delay 2.0)
  (bind _returnvalue (UserInterface|CreateWidget "/Game/Hush/HUD/W_DeathMenu.W_DeathMenu_C"))
  (UserInterface|Viewport|AddtoViewport _returnvalue 0))

(event EventBeginPlay
  (Development|ExecuteConsoleCommand "ENABLEALLSCREENMESSAGES" 0))

(event EventTick
  (params (DeltaSeconds :type Float%20%28single-precision%29)))

(fn ConstructionScript)