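; Player controller for Hush that turns Enhanced Input into look, movement, crouch, sprint, flash, pause and interaction.
; Movement states drive footstep and breathing audio, and sprinting reports noise events.
; Crouch resizes the capsule on a timeline, with Tick retrying blocked uncrouches via capsule trace.
; Tick also line-traces for levers and gramophones to interact with, while custom events add or remove input mapping contexts.
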(event Custom|ModifyInteractIMC
  (params (IsEnabled :type Boolean))
  (bind _returnvalue (PlayerController|LocalPlayerSubsystems|GetEnhancedInputLocalPlayerSubsystem))
  (if IsEnabled
    (Input|AddMappingContext _returnvalue "/Game/Hush/Input/Keyboard/Using/IMC_Interact.IMC_Interact" 0 "(bIgnoreAllPressedKeysUntilRelease=True,bForceImmediately=False)")
    (else
      (Input|RemoveMappingContext _returnvalue "/Game/Hush/Input/Keyboard/Using/IMC_Interact.IMC_Interact" "(bIgnoreAllPressedKeysUntilRelease=True,bForceImmediately=False)"))))

(event Custom|IsPlayerOnlyWalking
  (bind _breathingaudio (Variables|Default|GetBreathingAudio))
  (bind _breathingaudio_2 (Variables|Default|GetBreathingAudio))
  (bind _breathingaudio_3 (Variables|Default|GetBreathingAudio))
  (if (Variables|Default|GetisRunning)
    (if (not (Variables|Default|GetIsPlayingRun))
      (Audio|Components|Audio|SetSound (Variables|Default|GetWalkAudio) "/Game/Hush/Sound/Player/running_v1.running_v1")
      (Variables|Default|SetIsPlayingRun true)
      (Variables|Default|SetIsPlayingCrouch false)
      (Variables|Default|SetIsPlayingWalk false)
      (Utilities|FlowControl|Delay 1.5)
      (Audio|Components|Audio|SetSound _breathingaudio_3 "/Game/Hush/Sound/Player/man_breathing.man_breathing")
      (Audio|Components|Audio|FadeIn _breathingaudio_3 1.0 1.0 0.0 "Linear" :!class /Script/Engine.AudioComponent))
    (elif (Variables|Default|GetisCrouching)
      (if (not (Variables|Default|GetIsPlayingCrouch))
        (Audio|Components|Audio|SetSound (Variables|Default|GetWalkAudio) "/Game/Hush/Sound/Player/Walking_Crouched.Walking_Crouched")
        (Variables|Default|SetIsPlayingRun false)
        (Variables|Default|SetIsPlayingCrouch true)
        (Variables|Default|SetIsPlayingWalk false)
        (Utilities|FlowControl|Delay 3.0)
        (Audio|Components|Audio|SetSound _breathingaudio "/Game/Hush/Sound/Player/man_breathing_slowly.man_breathing_slowly")
        (Audio|Components|Audio|FadeIn _breathingaudio 1.0 1.0 0.0 "Linear" :!class /Script/Engine.AudioComponent))
      (elif (not (Variables|Default|GetIsPlayingWalk))
        (Audio|Components|Audio|SetSound (Variables|Default|GetWalkAudio) "/Game/Hush/Sound/Player/walking.walking")
        (Variables|Default|SetIsPlayingRun false)
        (Variables|Default|SetIsPlayingCrouch false)
        (Variables|Default|SetIsPlayingWalk true)
        (Utilities|FlowControl|Delay 3.0)
        (Audio|Components|Audio|SetSound _breathingaudio_2 "/Game/Hush/Sound/Player/man_breathing_slowly.man_breathing_slowly")
        (Audio|Components|Audio|FadeIn _breathingaudio_2 1.0 1.0 0.0 "Linear" :!class /Script/Engine.AudioComponent)))))

(event Custom|ModifyHoldIMC
  (params (IsEnabled :type Boolean))
  (bind _returnvalue (PlayerController|LocalPlayerSubsystems|GetEnhancedInputLocalPlayerSubsystem))
  (if IsEnabled
    (Input|AddMappingContext _returnvalue "/Game/Hush/Input/Keyboard/Using/IMC_Hold.IMC_Hold" 0 "(bIgnoreAllPressedKeysUntilRelease=True,bForceImmediately=False)")
    (else
      (Input|RemoveMappingContext _returnvalue "/Game/Hush/Input/Keyboard/Using/IMC_Hold.IMC_Hold" "(bIgnoreAllPressedKeysUntilRelease=True,bForceImmediately=False)"))))

(event Custom|ModifyKeyboardIMC
  (bind _walkaudio (Variables|Default|GetWalkAudio))
  (Input|RemoveMappingContext (PlayerController|LocalPlayerSubsystems|GetEnhancedInputLocalPlayerSubsystem) "/Game/Hush/Input/Keyboard/IMC_Keyboard.IMC_Keyboard" "(bIgnoreAllPressedKeysUntilRelease=True,bForceImmediately=False)")
  (Utilities|IsValid _walkaudio
    (:Is%20Valid
      (Audio|Components|Audio|Stop _walkaudio))))

(event Custom|ModifyMouseIMC
  (Input|RemoveMappingContext (PlayerController|LocalPlayerSubsystems|GetEnhancedInputLocalPlayerSubsystem) "/Game/Hush/Input/Mouse/IMC_Mouse.IMC_Mouse" "(bIgnoreAllPressedKeysUntilRelease=True,bForceImmediately=False)"))

(event Input|EnhancedActionEvents|EnhancedInputActionIA_Movement
  (params (ActionValue :type Vector%202D%20Structure) (ElapsedSeconds :type Float%20%28double-precision%29) (TriggeredSeconds :type Float%20%28double-precision%29) (InputAction :type Input%20Action%20Object%20Reference :default "/Game/Hush/Input/Keyboard/IA_Movement.IA_Movement"))
  (bind _returnvalue (Pawn|GetControlRotation :!class /Script/Engine.Controller))
  (bind _returnvalue_2 (Game|Player|GetPlayerPawn 0))
  ;[1 1 1] Movement
  (:Triggered
    (if (Variables|Default|GetcanMove)
      (Variables|Default|SetIsMoving true)
      (Pawn|Input|AddMovementInput _returnvalue_2 (* (Math|Vector|GetRightVector (Math|Rotator|MakeRotator (.roll _returnvalue) 0.0 (.yaw _returnvalue))) (Variables|Default|GetmovSpeed)) (.x ActionValue) false)
      (Pawn|Input|AddMovementInput _returnvalue_2 (* (Math|Vector|GetForwardVector (Math|Rotator|MakeRotator 0.0 0.0 (.yaw _returnvalue))) (Variables|Default|GetmovSpeed)) (.y ActionValue) false)
      (Class|LegacyCameraShake|StartLegacyCameraShake (Game|GetPlayerCameraManager 0) "/Game/Hush/Blueprints/BP_CameraShake.BP_CameraShake_C" 1.0 "CameraLocal" "0, 0, 0")
      (CallFunction|IsPlayerOnlyWalking)))
  (:Started
    (bind _returnvalue_3 (Audio|SpawnSound2D "/Game/Hush/Sound/Player/walking.walking" 1.0 1.0 0.0 0))
    (Variables|Default|SetWalkAudio _returnvalue_3)
    (Variables|Default|SetIsPlayingWalk true)
    (Audio|Components|Audio|SetSound (Variables|Default|GetBreathingAudio) "/Game/Hush/Sound/Player/man_breathing_slowly.man_breathing_slowly"))
  (:Completed
    (Variables|Default|SetIsMoving false)
    (Utilities|IsValid (Variables|Default|GetWalkAudio)
      (:Is%20Valid
        (Audio|Components|Audio|Stop (Variables|Default|GetWalkAudio))
        (Utilities|FlowControl|Delay 3.0)
        (Utilities|FlowControl|Delay 0.5)
        (Audio|Components|Audio|SetSound (Variables|Default|GetBreathingAudio) "/Game/Hush/Sound/Player/man_breathing_idle.man_breathing_idle")))))

(event Input|EnhancedActionEvents|EnhancedInputActionIA_MouseMovement
  (params (ActionValue :type Vector%202D%20Structure) (ElapsedSeconds :type Float%20%28double-precision%29) (TriggeredSeconds :type Float%20%28double-precision%29) (InputAction :type Input%20Action%20Object%20Reference :default "/Game/Hush/Input/Mouse/IA_MouseMovement.IA_MouseMovement"))
  (bind _sensvar (Variables|Default|GetsensVar))
  ;[1 1 1] Mouse Movement
  (:Triggered
    (if (Variables|Default|GetcanMove)
      (Class|PlayerController|AddYawInput (* (.x ActionValue) _sensvar))
      (Class|PlayerController|AddPitchInput (* (.y ActionValue) _sensvar)))))

(event Input|EnhancedActionEvents|EnhancedInputActionIA_Crouch
  (params (ActionValue :type Boolean) (ElapsedSeconds :type Float%20%28double-precision%29) (TriggeredSeconds :type Float%20%28double-precision%29) (InputAction :type Input%20Action%20Object%20Reference :default "/Game/Hush/Input/Keyboard/IA_Crouch.IA_Crouch"))
  ;[1 1 1] Crouch
  (:Triggered
    (if (Variables|Default|GetcanMove)
      (Variables|Default|SetisCrouching true)
      (bind _returnvalue (Actor|GetActorOfClass "/Game/Hush/Blueprints/BP_Char.BP_Char_C"))
      (Variables|/Script/Engine.CharacterMovementComponent|SetMaxWalkSpeed (Actor|GetComponentbyClass _returnvalue "/Script/Engine.CharacterMovementComponent") 3e+02)
      (bind _crouch (Timeline|TL_Crouch Play)
        (:Update
          (bind _returnvalue_2 (Actor|GetActorOfClass "/Game/Hush/Blueprints/BP_Char.BP_Char_C"))
          (Components|Capsule|SetCapsuleHalfHeight (Variables|/Script/Engine.Character|GetCapsuleComponent _returnvalue_2) (Math|Float|Lerp 88.0 44.0 _crouch) true)))))
  (:Started
    (Audio|PlaySound2D "/Game/Hush/Sound/Player/crouch_short.crouch_short" 1.0 1.0 0.1 0 0))
  (:Completed
    (bind _returnvalue_3 (Actor|GetActorOfClass "/Game/Hush/Blueprints/BP_Char.BP_Char_C"))
    (bind _returnvalue_4 (Collision|CapsuleTraceByChannel (+ (Transformation|GetWorldLocation (Variables|/Script/Engine.Character|GetMesh _returnvalue_3)) "0.000000,0.000000,44.000000") (+ (Transformation|GetWorldLocation (Variables|/Script/Engine.Character|GetMesh _returnvalue_3)) "0.000000,0.000000,44.000000") 34.0 88.0 "TraceTypeQuery1" false 0 "None"))
    (if _returnvalue_4
      (Variables|Default|SetcantUncrouch true)
      (else
        (Variables|Default|SetisCrouching false)
        (bind _returnvalue_5 (Actor|GetActorOfClass "/Game/Hush/Blueprints/BP_Char.BP_Char_C"))
        (Variables|/Script/Engine.CharacterMovementComponent|SetMaxWalkSpeed (Actor|GetComponentbyClass _returnvalue_5 "/Script/Engine.CharacterMovementComponent") 5e+02)
        (Audio|PlaySound2D "/Game/Hush/Sound/Player/uncrouch_short.uncrouch_short" 1.0 1.0 0.0 0 0)
        (Timeline|TL_Crouch Reverse)))))

(event Input|EnhancedActionEvents|EnhancedInputActionIA_Run
  (params (ActionValue :type Boolean) (ElapsedSeconds :type Float%20%28double-precision%29) (TriggeredSeconds :type Float%20%28double-precision%29) (InputAction :type Input%20Action%20Object%20Reference :default "/Game/Hush/Input/Keyboard/IA_Run.IA_Run"))
  (bind _returnvalue (Game|GetPlayerCharacter 0))
  (bind _returnvalue_2 (Game|GetPlayerCharacter 0))
  (bind _charactermovement (Variables|/Script/Engine.Character|GetCharacterMovement _returnvalue))
  ;[1 1 1] Sprint
  (:Triggered
    (if (Variables|Default|GetIsMoving)
      (if (not (Variables|Default|GetisCrouching))
        (Variables|Default|SetisRunning true)
        (Variables|/Script/Engine.CharacterMovementComponent|SetMaxWalkSpeed _charactermovement 8e+02)
        (Class|AISenseHearing|ReportNoiseEvent (Transformation|GetActorLocation _returnvalue_2) 1.0 _returnvalue_2 0.0 "None"))
      (elif (not (Variables|Default|GetisCrouching))
        (Variables|Default|SetisRunning false)
        (Variables|Default|SetIsPlayingRun false))))
  (:Completed
    (Variables|Default|SetisRunning false)
    (Variables|/Script/Engine.CharacterMovementComponent|SetMaxWalkSpeed _charactermovement 5e+02)))

(event Input|EnhancedActionEvents|EnhancedInputActionIA_Pause
  (params (ActionValue :type Boolean) (ElapsedSeconds :type Float%20%28double-precision%29) (TriggeredSeconds :type Float%20%28double-precision%29) (InputAction :type Input%20Action%20Object%20Reference :default "/Game/Hush/Input/Keyboard/IA_Pause.IA_Pause"))
  (bind _returnvalue (Game|GetPlayerController 0))
  (bind (_sizex _sizey) (HUD|GetViewportSize _returnvalue))
  ;[1 1 1] Pause
  (:Triggered
    (if (Variables|Default|GetisInMenu)
      (Viewport|RemoveAllWidgets)
      (Variables|Default|SetbShowMouseCursor false)
      (Variables|Default|SetisPaused false)
      (Variables|Default|SetcanMove true)
      (Variables|Default|SetisInMenu false)
      (Input|SetInputModeGameOnly (Game|GetPlayerController 0) false)
      (bind _returnvalue_2 (UserInterface|CreateWidget "/Game/Hush/HUD/W_Crosshair.W_Crosshair_C"))
      (UserInterface|Viewport|AddtoViewport _returnvalue_2 0)
      (elif (Variables|Default|GetisPaused)
        (Variables|Default|SetisPaused false)
        (Variables|Default|SetcanMove true)
        (Variables|Default|SetisInMenu false)
        (Widget|RemovefromParent (stale _returnvalue_3))
        (Variables|Default|SetbShowMouseCursor false)
        (Input|SetInputModeGameOnly _returnvalue false)
        (else
          (Variables|Default|SetisPaused true)
          (Variables|Default|SetcanMove false)
          (Variables|Default|SetisInMenu true)
          (bind _returnvalue_3 (UserInterface|CreateWidget "/Game/Hush/HUD/W_PauseMenu.W_PauseMenu_C"))
          (UserInterface|Viewport|AddtoViewport _returnvalue_3 0)
          (Variables|Default|SetbShowMouseCursor true)
          (Input|SetInputModeGameandUI _returnvalue 0 "DoNotLock" true false)
          (Class|PlayerController|SetMouseLocation _returnvalue (/ _sizex 2) (/ _sizey 2)))))))

(event Input|EnhancedActionEvents|EnhancedInputActionIA_Flash
  (params (ActionValue :type Boolean) (ElapsedSeconds :type Float%20%28double-precision%29) (TriggeredSeconds :type Float%20%28double-precision%29) (InputAction :type Input%20Action%20Object%20Reference :default "/Game/Hush/Input/Mouse/IA_Flash.IA_Flash"))
  (:Started
    (if (not (Variables|Default|GetisPaused))
      (bind _returnvalue (Actor|GetActorOfClass "/Game/Hush/Blueprints/BP_Char.BP_Char_C"))
      (Default|EventFlash (Actor|GetComponentbyClass _returnvalue "/Game/Hush/Blueprints/Component/AC_Flash.AC_Flash_C")))))

(event Input|EnhancedActionEvents|EnhancedInputActionIA_HoldInteract
  (params (ActionValue :type Boolean) (ElapsedSeconds :type Float%20%28double-precision%29) (TriggeredSeconds :type Float%20%28double-precision%29) (InputAction :type Input%20Action%20Object%20Reference :default "/Game/Hush/Input/Keyboard/Using/IA_HoldInteract.IA_HoldInteract"))
  (:Triggered
    (Default|ColorLight (stale EventTick _asbp_lever))
    (Default|EndHoldingLever (stale EventTick _asbp_lever)))
  (:Started
    (Default|StartPullingLever (stale EventTick _asbp_lever)))
  (:Ongoing
    (Utilities|FlowControl|Delay 0.1)
    (Default|UpdateHoldWidget (stale EventTick _asbp_lever)))
  (:Canceled
    (Default|CancelHolding (stale EventTick _asbp_lever))))

(event Input|EnhancedActionEvents|EnhancedInputActionIA_Interact
  (params (ActionValue :type Boolean) (ElapsedSeconds :type Float%20%28double-precision%29) (TriggeredSeconds :type Float%20%28double-precision%29) (InputAction :type Input%20Action%20Object%20Reference :default "/Game/Hush/Input/Keyboard/Using/IA_Interact.IA_Interact"))
  ;[1 1 1] Linetrace
  (:Triggered
    (if (not (Variables|/Game/Hush/Blueprints/MapGenerating/BP_Gramophone.BP_Gramophone_C|GetSoundIsPlaying (stale EventTick _asbp_gramophone)))
      (Default|SwitchonGramophone (stale EventTick _asbp_gramophone)))))

(event Input|EnhancedActionEvents|EnhancedInputActionIA_AllLeversPulled
  (params (ActionValue :type Boolean) (ElapsedSeconds :type Float%20%28double-precision%29) (TriggeredSeconds :type Float%20%28double-precision%29) (InputAction :type Input%20Action%20Object%20Reference :default "/Game/Hush/Input/Debug/IA_AllLeversPulled.IA_AllLeversPulled"))
  (:Started
    (bind _returnvalue (Actor|GetActorOfClass "/Game/Hush/Gamemodes/GM_Testing.GM_Testing_C"))
    (Default|AllLeversActivated _returnvalue)))

(event EventBeginPlay
  (bind _returnvalue (PlayerController|LocalPlayerSubsystems|GetEnhancedInputLocalPlayerSubsystem))
  ;[1 1 1] Setup
  (Utilities|IsValid _returnvalue
    (:Is%20Valid
      (Variables|Default|SetcanMove true)
      (Input|AddMappingContext _returnvalue "/Game/Hush/Input/Keyboard/IMC_Keyboard.IMC_Keyboard" 0 "(bIgnoreAllPressedKeysUntilRelease=True,bForceImmediately=False)")
      (Input|AddMappingContext _returnvalue "/Game/Hush/Input/Mouse/IMC_Mouse.IMC_Mouse" 0 "(bIgnoreAllPressedKeysUntilRelease=True,bForceImmediately=False)")
      (Actor|GetActorOfClass "/Game/Hush/Blueprints/BP_Char.BP_Char_C")
      (Utilities|Casting|CastToBP_Char (Game|Player|GetPlayerPawn 0))
      (bind _returnvalue_2 (Audio|SpawnSound2D "/Game/Hush/Sound/Player/man_breathing_idle.man_breathing_idle" 1.0 1.0 0.0 0))
      (Variables|Default|SetBreathingAudio _returnvalue_2))))

(event EventTick
  (params (DeltaSeconds :type Float%20%28single-precision%29))
  (Utilities|FlowControl|Sequence
    (:then_0
      (bind (_actorhit _hit) (CallFunction|Trace))
      (if _hit
        (bind _asbp_lever (Utilities|Casting|CastToBP_Lever _actorhit)
          (:then
            (Default|LeverDetected _asbp_lever))
          (:CastFailed
            (bind _asbp_gramophone (Utilities|Casting|CastToBP_Gramophone _actorhit))
            (Default|GramophoneIsDetected _asbp_gramophone)))
        (else
          (bind _outactors (Actor|GetAllActorsOfClass "/Game/Hush/Blueprints/MapGenerating/BP_Lever.BP_Lever_C"))
          (for _array_element _outactors
            (Default|LeverNotDetected _array_element))
          (bind _outactors_2 (Actor|GetAllActorsOfClass "/Game/Hush/Blueprints/MapGenerating/BP_Gramophone.BP_Gramophone_C"))
          (for _array_element_2 _outactors_2
            (Default|GramophoneNotDetected _array_element_2)))))
    (:then_1
      ;[1 1 1] Uncrouch Check
      (if (Variables|Default|GetcantUncrouch)
        (bind _returnvalue (Actor|GetActorOfClass "/Game/Hush/Blueprints/BP_Char.BP_Char_C"))
        (bind _returnvalue_2 (Collision|CapsuleTraceByChannel (+ (Transformation|GetWorldLocation (Variables|/Script/Engine.Character|GetMesh _returnvalue)) "0.000000,0.000000,44.000000") (+ (Transformation|GetWorldLocation (Variables|/Script/Engine.Character|GetMesh _returnvalue)) "0.000000,0.000000,44.000000") 34.0 88.0 "TraceTypeQuery1" false 0 "None"))
        (if (not _returnvalue_2)
          (Variables|Default|SetcantUncrouch false)
          ;[1 1 1] Crouch
          (Variables|Default|SetisCrouching false)
          (bind _returnvalue_3 (Actor|GetActorOfClass "/Game/Hush/Blueprints/BP_Char.BP_Char_C"))
          (Variables|/Script/Engine.CharacterMovementComponent|SetMaxWalkSpeed (Actor|GetComponentbyClass _returnvalue_3 "/Script/Engine.CharacterMovementComponent") 5e+02)
          (Audio|PlaySound2D "/Game/Hush/Sound/Player/uncrouch_short.uncrouch_short" 1.0 1.0 0.0 0 0)
          (bind _crouch (Timeline|TL_Crouch Reverse)
            (:Update
              (bind _returnvalue_4 (Actor|GetActorOfClass "/Game/Hush/Blueprints/BP_Char.BP_Char_C"))
              (Components|Capsule|SetCapsuleHalfHeight (Variables|/Script/Engine.Character|GetCapsuleComponent _returnvalue_4) (Math|Float|Lerp 88.0 44.0 _crouch) true))))))))

(fn ConstructionScript)

(fn Trace
  (bind _asbp_char (Utilities|Casting|CastToBP_Char (Game|GetPlayerCharacter 0)))
  (bind (_outhit _returnvalue) (Collision|LineTraceByChannel (Math|Vector|MakeVector (.x (Transformation|GetActorLocation _asbp_char)) (.y (Transformation|GetActorLocation _asbp_char)) (+ (.z (Transformation|GetActorLocation _asbp_char)) (Variables|Default|GetlineTraceHeight))) (Math|Vector|MakeVector (+ (.x (Transformation|GetActorLocation _asbp_char)) (.x (* (Math|Vector|GetForwardVector (Pawn|GetControlRotation _asbp_char :!class /Script/Engine.Pawn)) 2e+03))) (+ (.y (Transformation|GetActorLocation _asbp_char)) (.y (* (Math|Vector|GetForwardVector (Pawn|GetControlRotation _asbp_char :!class /Script/Engine.Pawn)) 2e+03))) (+ (.z (Transformation|GetActorLocation _asbp_char)) (.z (* (Math|Vector|GetForwardVector (Pawn|GetControlRotation _asbp_char :!class /Script/Engine.Pawn)) 2e+03)))) "TraceTypeQuery3" false 0 "None"))
  (return (.HitActor (Collision|BreakHitResult _outhit)) _returnvalue))